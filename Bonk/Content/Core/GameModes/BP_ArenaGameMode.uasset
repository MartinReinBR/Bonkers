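; Arena game mode that runs timed rounds, awards player money and rotates randomly chosen streamed levels.
; Round events reset the countdown and kill stats, run a looping one-second timer that ends the round at zero, and play win sounds.
; Round end pays itemized money for completion, kills and bounties.
; Entering the shop destroys weapon actors and loads a random level from the map's valid entries.
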(event `self.ReceiveBeginPlay`
  (`|ExecutionSequence`
    (:`then_0`
      (add `self.OnPreRoundStart` (`|CreateDelegate` :!event `OnPreRoundStart_Event_0`)))
    (:`then_1`
      (add `self.OnRoundStart` (`|CreateDelegate` :!event `OnRoundStart_Event`)))
    (:`then_2`
      (add `self.OnRoundEnd` (`|CreateDelegate` :!event `OnRoundEnd_Event`)))
    (:`then_3`
      (`self.LoadRandomDynamicLevel`))))

(event `OnTeamMatchWin_Event_0` :!signature `self.OnTeamMatchWin`
  (params (TeamName :type "Text (by ref)"))
  (add `self.OnTeamMatchWin` (delegate `OnTeamMatchWin_Event_0`))
  (`GameplayStatics.PlaySound2D` "/Game/SoundEffects/Win_Match.Win_Match" 1.0 1.0 0.0 null null))

(event `OnPreRoundStart_Event_0` :!signature `self.OnPreRoundStart`
  (params (RoundNumber :type Integer))
  (bind _output_get (set `self.Time` 180))
  (`self.OnTimeUpdated` _output_get)
  (add `self.OnShopEntered` (`|CreateDelegate` :!event `OnShopEntered_Event`)))

(event `OnRoundEnd_Event` :!signature `self.OnRoundEnd`
  (params (RoundNumber :type Integer))
  (bind _moneyround (`self.MoneyRound`))
  (`|ExecutionSequence`
    (:`then_0`
      ;[1 1 1] Award players their money
      (for _array_element (`self.GetPlayers`)
        (set `BonkPlayer.InitialRoundMoney` (`BonkPlayer.PlayerMoney` _array_element) _array_element)
        (bind _moneysources (`BonkPlayer.MoneySources` _array_element))
        (`KismetArrayLibrary.Array_Clear` _moneysources)
        (`KismetArrayLibrary.Array_Add` _moneysources (make `MoneySource` "Round complete" _moneyround))
        (bind _killcount (`BonkPlayer.KillCount` _array_element))
        (bind _returnvalue (* _killcount (`self.MoneyKill`)))
        (`KismetArrayLibrary.Array_Add` _moneysources (make `MoneySource` (`|FormatText` "{KillCount} {Text}" _killcount (select `bool` (== _killcount 1) :`false` "Kills" :`true` "Kill" :!type "Text")) _returnvalue))
        (bind _bountycount (`BonkPlayer.BountyCount` _array_element))
        (bind _returnvalue_2 (* _bountycount (`self.MoneyBounty`)))
        (`KismetArrayLibrary.Array_Add` _moneysources (make `MoneySource` (`|FormatText` "{BountyCount} {Text}" _bountycount (select `bool` (== _bountycount 1) :`false` "Collected bounties" :`true` "Collected bounty" :!type "Text")) _returnvalue_2))
        (`BonkPlayer.AddMoney` _array_element (+ _returnvalue _returnvalue_2 _moneyround))
        (`KismetSystemLibrary.K2_ClearAndInvalidateTimerHandle` (`self.RoundTimer`))))
    (:`then_1`
      (`GameplayStatics.PlaySound2D` "/Game/SoundEffects/Win_round.Win_round" 2.0 1.0 0.0 null null))))

(event `OnRoundStart_Event` :!signature `self.OnRoundStart`
  (params (RoundNumber :type Integer))
  ;[1 1 1] Super rough timer, refactor later if needed
  ;;[1 1 1] Reset round kill stats
  (for _array_element (`self.GetPlayers`)
    (set `BonkPlayer.KillCount` 0 _array_element)
    (set `BonkPlayer.BountyCount` 0 _array_element)
    (`KismetArrayLibrary.Array_Clear` (`BonkPlayer.KilledPlayers` _array_element))
    (bind _returnvalue (`KismetSystemLibrary.K2_SetTimerDelegate` (delegate `CustomEvent_0`) 1.0 true))
    (set `self.RoundTimer` _returnvalue)))

(event `CustomEvent_0`
  ;[1 1 1] Super rough timer, refactor later if needed
  (bind _result (`/Engine/EditorBlueprintResources/StandardMacros.DecrementInt` (`self.Time`))
    (:`  `
      (`self.OnTimeUpdated` _result)
      (if (<= (`self.Time`) 0)
        (`KismetSystemLibrary.K2_ClearAndInvalidateTimerHandle` (`self.RoundTimer`))
        (`KismetSystemLibrary.Delay` 1.0)
        (`self.EndRound`)))))

(event `LoadRandomDynamicLevel`
  (bind _currentdynamiclevel (`self.CurrentDynamicLevel`))
  ;[1 1 1] Loading random dynamic level
  (if (and (`KismetSystemLibrary.IsValidSoftObjectReference` (`self.CurrentDynamicLevel`)) (`self.ShouldUnloadDynamicLevel`))
    (`GameplayStatics.UnloadStreamLevelBySoftObjectPtr` _currentdynamiclevel true))
  (`GameplayStatics.LoadStreamLevelBySoftObjectPtr` (`self.GetRandomDynamicLevel` _currentdynamiclevel) true)
  (if (`KismetSystemLibrary.IsValidSoftObjectReference` (`self.CurrentDynamicLevel`))
    (`KismetSystemLibrary.PrintString` "Dynaic")))

(event `OnShopEntered_Event`
  (`|ExecutionSequence`
    (:`then_0`
      (bind _outactors (`GameplayStatics.GetAllActorsOfClass` "/Game/Core/Interactable/Weapons/BP_Weap_Base.BP_Weap_Base_C"))
      (for _array_element _outactors
        (`self.K2_DestroyActor` _array_element)))
    (:`then_1`
      (`self.LoadRandomDynamicLevel`))))

(fn `GetRandomDynamicLevel`
  (params (CurrentDynamicLevel1 :type "World Soft Object Reference"))
  (returns (CurrentDynamicLevel :type "World Soft Object Reference"))
  (locals (PreviousDynamicLevel :type "World Soft Object Reference") (ValidDynamicLevels :type "Array of World Soft Object Reference"))
  (`|ExecutionSequence`
    (:`then_0`
      ;[1 1 1] Get a list of maps we can choose from
      (if (`KismetSystemLibrary.IsValidSoftObjectReference` CurrentDynamicLevel1)
        (set `local.PreviousDynamicLevel` CurrentDynamicLevel1)))
    (:`then_1`
      (set `local.ValidDynamicLevels` (`self.GetValidDynamicLevels`)))
    (:`then_2`
      (`|ExecutionSequence`
        (:`then_0`
          (if (not (`KismetArrayLibrary.Array_Contains` (`local.ValidDynamicLevels`) (`local.PreviousDynamicLevel`)))
            (`KismetArrayLibrary.Array_RemoveItem` (`local.ValidDynamicLevels`) (`local.PreviousDynamicLevel`))))
        (:`then_1`
          (set `self.CurrentDynamicLevel` (`KismetArrayLibrary.Array_Random` (`local.ValidDynamicLevels`))))
        (:`then_2`
          (return (`self.CurrentDynamicLevel`)))))))

(fn `GetValidDynamicLevels`
  (returns (AllValidDynamicLevels :type "Array of World Soft Object Reference"))
  (locals (ValidDynamicLevels :type "Array of World Soft Object Reference"))
  (`KismetArrayLibrary.Array_Clear` (`local.ValidDynamicLevels`))
  (bind _values (`BlueprintMapLibrary.Map_Values` (`self.AllDynamicLevels`)))
  (for (_array_element _array_index) _values
    (if (== _array_element 0)
      (bind _keys (`BlueprintMapLibrary.Map_Keys` (`self.AllDynamicLevels`)))
      (`KismetArrayLibrary.Array_Add` (`local.ValidDynamicLevels`) (`|GetArrayItem` _keys _array_index))))
  (return (`local.ValidDynamicLevels`)))

(fn `UserConstructionScript`)