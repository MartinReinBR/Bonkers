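; BP_BonkCamera is the Bonk game camera, following player pawns during rounds and zooming out when the audience spawns a weapon.
; It binds to round events, setting all BonkPlayerPawns as follow targets at pre-round start, then clearing them and teleporting back to its initial location at round end.
; BonkAudience's weapon-spawn event starts the zoom-out sequence.
; The construction script draws a temporary debug box sized from the camera bounds.
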(event `self.ReceiveBeginPlay`
  (bind _returnvalue (`BonkGameModeBase.Get`))
  (`/Engine/EditorBlueprintResources/StandardMacros.IsValid` _returnvalue
    (:`Is Valid`
      (add `BonkGameModeBase.OnPreRoundStart` _returnvalue (delegate `AssignPlayers`))
      (add `BonkGameModeBase.OnRoundEnd` _returnvalue (delegate `RemovePlayers`)))
    (:`Is Not Valid`
      _))
  (bind _returnvalue_2 (`GameplayStatics.GetActorOfClass` "/Script/Bonk.BonkAudience"))
  (`/Engine/EditorBlueprintResources/StandardMacros.IsValid` _returnvalue_2
    (:`Is Valid`
      (add `BonkAudience.OnWeaponSpawned` _returnvalue_2 (delegate `OnWeaponSpawned_Event_0`)))))

(event `AssignPlayers`
  (params (RoundNumber :type Integer))
  (bind _outactors (`GameplayStatics.GetAllActorsOfClass` "/Script/Bonk.BonkPlayerPawn"))
  (`self.SetFollowTargets` _outactors))

(event `OnWeaponSpawned_Event_0`
  (`self.StartZoomoutSequence`))

(event `RemovePlayers`
  (params (RoundNumber :type Integer))
  (`self.ClearFollowTargets`)
  (`self.K2_SetActorLocation` (`self.InitialLocation`) false true))

(fn `UserConstructionScript`
  (`KismetSystemLibrary.DrawDebugBox` (`self.K2_GetActorLocation`) (+ (`KismetMathLibrary.Vector_GetAbs` (`self.CameraMinBounds`)) (`self.CameraMaxBounds`)) (struct :`G` 0.017362 :`B` 1.0 :`A` 1.0) (struct) 10.0 10.0))