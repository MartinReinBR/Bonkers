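; BP_BonkAudience is an audience Blueprint that periodically throws items toward a point in a box while a round is running.
; BeginPlay binds to round start and end events to toggle activity, or stays active if the object providing those events is invalid.
; While active, Tick accumulates time, calls ThrowItemToPointInBox once the wait elapses, then picks a new random interval between the configured spawn limits.
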(event `self.ReceiveBeginPlay`
  (bind _returnvalue (`BonkGameModeBase.Get`))
  (`/Engine/EditorBlueprintResources/StandardMacros.IsValid` _returnvalue
    (:`Is Valid`
      (add `BonkGameModeBase.OnRoundStart` _returnvalue (delegate `OnRoundStart`))
      (add `BonkGameModeBase.OnRoundEnd` _returnvalue (delegate `OnRoundEnd`)))
    (:`Is Not Valid`
      (set `self.IsActive` true)))
  (set `self.WaitTime` (`KismetMathLibrary.RandomFloatInRange` (`self.MinTimeBetweenSpawns`) (`self.MaxTimeBetweenSpawns`))))

(event `OnRoundStart`
  (params (RoundNumber :type Integer))
  (set `self.IsActive` true))

(event `OnRoundEnd`
  (params (RoundNumber :type Integer))
  (set `self.IsActive` false))

(event `self.ReceiveTick`
  (params (DeltaSeconds :type "Float (single-precision)"))
  (if (`self.IsActive`)
    (set `self.WaitTimer` (+ DeltaSeconds (`self.WaitTimer`)))
    (if (>= (`self.WaitTimer`) (`self.WaitTime`))
      (`self.ThrowItemToPointInBox`)
      (set `self.WaitTimer` 0.0)
      (set `self.WaitTime` (`KismetMathLibrary.RandomFloatInRange` (`self.MinTimeBetweenSpawns`) (`self.MaxTimeBetweenSpawns`))))))

(fn `UserConstructionScript`)