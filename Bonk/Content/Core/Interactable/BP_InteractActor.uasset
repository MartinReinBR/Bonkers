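; Base-style interacting actor that picks up items and attacks with them through BonkAbility and BonkItemInteract components.
; Pickup notifies the ability component, then tries a pickup on the interact component.
; Attack notifies the ability component, then activates tracing on the current interactable's BonkBonkerComponent, if present.
; Tick draws debug visuals: selected interactable name, range and view-cone lines from the dot-product limit, and spheres on overlapped interactables.
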(event `self.ReceiveTick`
  (params (DeltaSeconds :type "Float (single-precision)"))
  (bind _returnvalue (`self.K2_GetActorLocation`))
  (bind _returnvalue_2 (`self.K2_GetActorLocation`))
  (bind _returnvalue_3 (`self.K2_GetActorLocation`))
  (`|ExecutionSequence`
    (:`then_0`
      (`KismetSystemLibrary.PrintString` (`KismetSystemLibrary.GetDisplayName` (`BonkItemInteractComponent.SelectedInteractable` (`self.BonkItemInteract`))) true true (struct :`R` 1.0 :`G` 1.0 :`B` 1.0 :`A` 1.0) 0.0)
      (`KismetSystemLibrary.DrawDebugLine` _returnvalue (+ _returnvalue (* (`self.GetActorForwardVector`) (`BonkItemInteractComponent.Range` (`self.BonkItemInteract`)))) (struct :`B` 1.0 :`A` 1.0) 0.0 3.0)
      (`KismetSystemLibrary.DrawDebugLine` _returnvalue_2 (+ _returnvalue_2 (* (`KismetMathLibrary.RotateAngleAxis` (`self.GetActorForwardVector`) (`KismetMathLibrary.DegAcos` (`BonkItemInteractComponent.DotProductLimits` (`self.BonkItemInteract`))) (0.0 0.0 1.0)) (`BonkItemInteractComponent.Range` (`self.BonkItemInteract`)))) (struct :`R` 0.301961 :`G` 0.301961 :`B` 1.0 :`A` 1.0) 0.0 3.0)
      (`KismetSystemLibrary.DrawDebugLine` _returnvalue_3 (+ _returnvalue_3 (* (`KismetMathLibrary.RotateAngleAxis` (`self.GetActorForwardVector`) (* (`KismetMathLibrary.DegAcos` (`BonkItemInteractComponent.DotProductLimits` (`self.BonkItemInteract`))) -1.0) (0.0 0.0 1.0)) (`BonkItemInteractComponent.Range` (`self.BonkItemInteract`)))) (struct :`R` 0.301961 :`G` 0.301961 :`B` 1.0 :`A` 1.0) 0.0 3.0))
    (:`then_1`
      (for _array_element (`BonkItemInteractComponent.OverlappedInteractables` (`self.BonkItemInteract`))
        (`KismetSystemLibrary.DrawDebugSphere` (`self.K2_GetActorLocation` (`ActorComponent.GetOwner` _array_element)) 50.0 12 (struct :`G` 1.0 :`A` 1.0) 0.0 3.0)))))

(fn `Attack`
  (bind _returnvalue (`self.GetComponentByClass` (`ActorComponent.GetOwner` (`BonkItemInteractComponent.CurrentInteractable` (`self.BonkItemInteract`))) "/Script/Bonk.BonkBonkerComponent"))
  (`BonkAbilityComponent.OnAttack` (`self.BonkAbility`))
  (`/Engine/EditorBlueprintResources/StandardMacros.IsValid` _returnvalue
    (:`Is Valid`
      (`BonkBonkerComponent.ActivateTracing` _returnvalue true))))

(fn `Pickup`
  (`BonkAbilityComponent.OnPickup` (`self.BonkAbility`) null)
  (`BonkItemInteractComponent.TryPickup` (`self.BonkItemInteract`)))

(fn `UserConstructionScript`)