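; BP_FloatingNumber is a short-lived world actor that shows a floating damage or health number.
; On BeginPlay it passes its value to a WBP_FloatingNumber widget component as damage or health, then destroys itself after a brief delay.
; Each tick it turns the widget on yaw only to face the BP_BonkCamera found at startup.
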(event `self.ReceiveBeginPlay`
  (bind _value (`self.Value`))
  (bind _returnvalue (`GameplayStatics.GetActorOfClass` "/Game/Core/BP_BonkCamera.BP_BonkCamera_C"))
  (set `self.Camera` _returnvalue)
  (bind _aswbp_floating_number (cast `/Game/Widgets/WBP_FloatingNumber` (`WidgetComponent.GetUserWidgetObject` (`self.Widget`))))
  (set `self.UIRef` _aswbp_floating_number)
  (`PrimitiveComponent.SetCastShadow` (`self.Widget`) false)
  (if (`self.Damage?`)
    (`self.Damage` _value)
    (else
      (`self.Health` _value)))
  (`KismetSystemLibrary.Delay` 0.7)
  (`self.K2_DestroyActor`))

(event `self.ReceiveTick`
  (params (DeltaSeconds :type "Float (single-precision)"))
  (`self.LookAtCamera`))

(fn `Damage`
  (params (Value :type "Float (double-precision)"))
  (`/Game/Widgets/WBP_FloatingNumber.FloatDamage` (`self.UIRef`) Value))

(fn `Health`
  (params (Value :type "Float (double-precision)"))
  (`/Game/Widgets/WBP_FloatingNumber.FloatHealth` (`self.UIRef`) Value))

(fn `LookAtCamera`
  (bind _camera (`self.Camera`)
    (:`then`
      (bind (_returnvalue_roll _returnvalue_pitch _returnvalue_yaw) (`KismetMathLibrary.BreakRotator` (`KismetMathLibrary.FindLookAtRotation` (`SceneComponent.K2_GetComponentLocation` (`self.Widget`)) (`self.K2_GetActorLocation` _camera))))
      (`SceneComponent.K2_SetWorldRotation` (`self.Widget`) (`KismetMathLibrary.MakeRotator` 0.0 0.0 _returnvalue_yaw) false false))
    (:`else`)))

(fn `UserConstructionScript`)