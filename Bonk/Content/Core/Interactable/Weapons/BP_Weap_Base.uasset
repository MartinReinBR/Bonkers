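; Base weapon Blueprint for pickup items that hit bonkable targets, with selection highlighting and a locator marker.
; Until pickup or disabling, Tick floats a widget facing BP_BonkCamera in yaw and line-traces down to place a ground decal widget, with debug drawing.
; InteractableComponent selection tints material instances, restoring base colors on deselect; dropping clears the owner from ignored actors after a delay.
; BonkerComponent hits notify the holding player pawn and play force feedback.
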(event `self.ReceiveBeginPlay`
  (bind _returnvalue (`GameplayStatics.GetActorOfClass` "/Game/Core/BP_BonkCamera.BP_BonkCamera_C"))
  (set `self.Camera` _returnvalue)
  (set `self.WidgetActive` true)
  (`KismetSystemLibrary.K2_SetTimerDelegate` (`|CreateDelegate` :!event `DisableWidget`) (`self.UITimer`))
  (`PrimitiveComponent.SetCastShadow` (`self.Widget`) false)
  (`PrimitiveComponent.SetCastShadow` (`self.DecalWidget`) false))

(event `self.ReceiveTick`
  (params (DeltaSeconds :type "Float (single-precision)"))
  (bind _decalwidget (`self.DecalWidget`))
  (bind _widget (`self.Widget`))
  (bind _returnvalue (+ (* (`KismetMathLibrary.Vector_Up`) 250.0) (`SceneComponent.K2_GetComponentLocation` (`self.Middle`))))
  (if (`self.WidgetActive`)
    (`SceneComponent.SetVisibility` (`self.Widget`) true false)
    (`self.LookAtCamera`)
    (`SceneComponent.K2_SetWorldLocation` _widget _returnvalue false false)
    (`SceneComponent.SetWorldScale3D` _widget (0.6 0.6 0.6))
    (bind _outhit (`KismetSystemLibrary.LineTraceSingle` :`Start` _returnvalue :`End` (- (`SceneComponent.K2_GetComponentLocation` (`self.Middle`)) (* (`KismetMathLibrary.Vector_Up`) 200.0)) :`TraceChannel` "TraceTypeQuery3" :`DrawDebugType` "ForOneFrame"))
    (bind (_bblockinghit _binitialoverlap _time _distance _location _impactpoint) (`GameplayStatics.BreakHitResult` _outhit))
    (`KismetSystemLibrary.DrawDebugSphere` _impactpoint 25.0 12 (struct :`R` 1.0 :`A` 1.0) 0.0 3.0)
    (`SceneComponent.K2_SetWorldLocation` _decalwidget (+ _impactpoint (* (`KismetMathLibrary.Vector_Up`) 5.0)) false false)
    (`SceneComponent.SetWorldScale3D` _decalwidget (2.0 2.0 2.0))
    (`SceneComponent.K2_SetWorldRotation` (`self.DecalWidget`) (struct :`Pitch` 90.0 :`Yaw` 180.0) false false)
    (`SceneComponent.SetVisibility` (`self.DecalWidget`) true false)
    (else
      (`SceneComponent.SetVisibility` (`self.Widget`) false false)
      (`SceneComponent.SetVisibility` (`self.DecalWidget`) false false))))

(event `self.InteractableComponent.OnPickupResponse`
  (params (InteractComp :type "BonkItemInteractComponent Object Reference"))
  ;[1 1 1] Pickup events
  (set `self.WidgetActive` false))

(event `self.InteractableComponent.OnDropResponse`
  (params (InteractComp :type "BonkItemInteractComponent Object Reference"))
  ;[1 1 1] Pickup events
  (`KismetSystemLibrary.Delay` 0.5)
  (`KismetArrayLibrary.Array_RemoveItem` (`BonkBonkerComponent.ActorsToIgnore` (`self.BonkerComponent`)) (`ActorComponent.GetOwner` InteractComp)))

(event `self.InteractableComponent.OnSelect`
  ;[1 1 1] Selection events
  ;;[1 1 1] Material
  (for _array_element (`self.MaterialInstances`)
    (bind _returnvalue (`MaterialInstanceDynamic.K2_GetVectorParameterValue` _array_element "Param"))
    (bind (_r _g _b) (`KismetMathLibrary.BreakColor` _returnvalue))
    (`MaterialInstanceDynamic.SetVectorParameterValue` _array_element "Param" (`KismetMathLibrary.MakeColor` 1.0 (* (/ (+ _r _g _b) 3.0) 0.5)))))

(event `self.InteractableComponent.OnDeselect`
  ;[1 1 1] Selection events
  ;;[1 1 1] Material
  (for (_array_element _array_index) (`self.MaterialInstances`)
    (`MaterialInstanceDynamic.SetVectorParameterValue` _array_element "Param" (`|GetArrayItem` (`self.BaseColors`) _array_index))))

(event `self.BonkerComponent.OnHit`
  (params (BonkableComponent :type "BonkBonkableComponent Object Reference") (FHitResult :type "HitResult Structure"))
  (bind _returnvalue (`ActorComponent.GetOwner` BonkableComponent))
  (bind _asbp_bonk_player_pawn (cast `/Game/Player/BP_BonkPlayerPawn` (`BonkBonkerComponent.GetHoldingPlayer` (`self.BonkerComponent`))))
  (`/Game/Player/BP_BonkPlayerPawn.OnBonkerHit` _asbp_bonk_player_pawn _returnvalue)
  (`/Game/Player/BP_BonkPlayerPawn.PlayHitForceFeedBack` _asbp_bonk_player_pawn _returnvalue))

(event `DisableWidget`
  (set `self.WidgetActive` false))

(fn `LookAtCamera`
  (bind _camera (`self.Camera`)
    (:`then`
      (bind (_returnvalue_roll _returnvalue_pitch _returnvalue_yaw) (`KismetMathLibrary.BreakRotator` (`KismetMathLibrary.FindLookAtRotation` (`SceneComponent.K2_GetComponentLocation` (`self.Widget`)) (`self.K2_GetActorLocation` _camera))))
      (`SceneComponent.K2_SetWorldRotation` (`self.Widget`) (`KismetMathLibrary.MakeRotator` 0.0 0.0 _returnvalue_yaw) false false))
    (:`else`)))

(fn `UserConstructionScript`)