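; BP_Weap_Crate is an interactable crate weapon that can bonk and be bonked.
; On BeginPlay it makes its collider bonkable and excludes itself from its BonkerComponent's targets.
; Pickup turns off both bonk roles and enables actor tick, while drop turns both back on.
; After a short post-drop delay, it removes the dropper from the bonker's ignore list, making them a valid target again.
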(event `self.ReceiveBeginPlay`
  (`parent.ReceiveBeginPlay`)
  (`BonkBonkableComponent.SetPrimitiveComponent` (`self.BonkBonkable`) (`self.GetColliderComp`))
  (`BonkBonkableComponent.EnableBonkable` (`self.BonkBonkable`) true)
  (`KismetArrayLibrary.Array_Add` (`BonkBonkerComponent.ActorsToIgnore` (`self.BonkerComponent`)) self))

(event `self.ReceiveTick`
  (params (DeltaSeconds :type "Float (single-precision)"))
  (`parent.ReceiveTick` DeltaSeconds))

(event `self.InteractableComponent.OnPickupResponse`
  (params (InteractComp :type "BonkItemInteractComponent Object Reference"))
  (`BonkBonkableComponent.EnableBonkable` (`self.BonkBonkable`) false)
  (set `BonkBonkerComponent.bCanBonk` false (`self.BonkerComponent`))
  (`self.SetActorTickEnabled` true))

(event `self.InteractableComponent.OnDropResponse`
  (params (InteractComp :type "BonkItemInteractComponent Object Reference"))
  (`BonkBonkableComponent.EnableBonkable` (`self.BonkBonkable`) true)
  (set `BonkBonkerComponent.bCanBonk` true (`self.BonkerComponent`))
  (`KismetSystemLibrary.Delay` 0.5)
  (`KismetArrayLibrary.Array_RemoveItem` (`BonkBonkerComponent.ActorsToIgnore` (`self.BonkerComponent`)) (`ActorComponent.GetOwner` InteractComp)))

(fn `UserConstructionScript`
  (`parent.UserConstructionScript`))