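; Player pawn for a team-colored brawler: picks up, swings and throws weapons, gets knocked around and tracks kills for a bounty display.
; PlayerInfo supplies stats to AbilityComp, while interact and bonkable component events drive montages, sounds, rumble, VFX and damage numbers.
; On destruction, a recent hit is credited to the damaging weapon's last holder through the game mode, otherwise counting as suicide.
; Tick interpolates hit tilt, projects a decal shadow and turns the bounty widget toward the camera.
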(event `self.ReceiveBeginPlay`
  (`|ExecutionSequence`
    (:`then_0`
      (add `self.OnDestroyed` (`|CreateDelegate` :!event `OnDestroyed_Event`))
      (add `self.OnDamaged` (`|CreateDelegate` :!event `OnDamaged_Event`))
      (add `self.OnBonkerHit` (`|CreateDelegate` :!event `OnBonkerHit_Event`))
      (add `self.OnHealed` (`|CreateDelegate` :!event `OnHealed_Event`)))
    (:`then_1`
      (set `self.bCanAttack` true))
    (:`then_2`
      (bind _returnvalue (`GameplayStatics.GetActorOfClass` "/Script/Engine.CameraActor"))
      (set `self.CameraActor` _returnvalue))
    (:`then_3`
      (`self.SetPawnColors`))
    (:`then_4`
      (`self.SetPlayerData`)
      (add `BonkPlayer.OnAddedKill` (`self.PlayerInfo`) (`|CreateDelegate` :!event `OnKilll_Event`)))
    (:`then_5`
      (`self.CreateVFX`))
    (:`then_6`
      (bind _returnvalue_2 (`GameplayStatics.GetActorOfClass` "/Game/Core/BP_BonkCamera.BP_BonkCamera_C"))
      (set `self.CameraRef` _returnvalue_2)
      (`PrimitiveComponent.SetCastShadow` (`self.Widget`) false))))

(event `InputAction|Start` :paused true
  (params (Key :type "Key Structure"))
  ;[1 1 1] Pause menu
  (:`Pressed`
    (bind _pausemenuref (`self.PauseMenuRef`)
      (:`then`
        (`/Game/Widgets/PauseMenu/WBP_PauseMenu.ClosePauseMenu` _pausemenuref)
        (set `self.PauseMenuRef` null))
      (:`else`
        (if (not (`GameplayStatics.IsGamePaused`))
          (bind _asplayer_controller (cast `PlayerController` (`self.GetController`)))
          (bind _returnvalue (`|CreateWidget` "/Game/Widgets/PauseMenu/WBP_PauseMenu.WBP_PauseMenu_C"))
          (bind _output_get (set `self.PauseMenuRef` _returnvalue))
          (`UserWidget.AddToViewport` _output_get 1)
          (`/Game/Widgets/PauseMenu/WBP_PauseMenu.GivePauseMenuFocus` _output_get (`GameplayStatics.GetPlayerControllerID` _asplayer_controller))
          (`GameplayStatics.SetGamePaused` true))))))

(event `OnDestroyed_Event` :!signature `self.OnDestroyed`
  (params (DestroyedActor :type "Actor Object Reference"))
  (`self.PlayDeathForceFeedback`)
  (bind _currentinteractable (`BonkItemInteractComponent.CurrentInteractable` (`self.InteractComp`))
    (:`then`
      (`self.K2_DestroyActor` (`ActorComponent.GetOwner` _currentinteractable)))
    (:`else`
      _))
  (`self.KillPlayer`)
  (`GameplayStatics.PlaySoundAtLocation` "/Game/SoundEffects/Player_Death.Player_Death" (`self.K2_GetActorLocation`) (struct) 0.4 1.0 0.0 "/Game/SoundEffects/Attenuation2.Attenuation2" null null null))

(event `self.OnAttack`
  (bind _interactcomp (`self.InteractComp`))
  ;[1 1 1] Player events
  (if (`BonkItemInteractComponent.bIsThrowing` _interactcomp)
    (`BonkItemInteractComponent.ResetThrow` _interactcomp)
    (set `self.bCanAttack` true)
    (`KismetSystemLibrary.PrintString` "RESET THROW")
    (else
      (`|PlayMontage` (`self.SkeletalComp`) "/Game/Animation/Montages/AM_Attack.AM_Attack" (* (`BonkAttribute.CurrentValue` (`BonkPlayer.AttackSpeed` (`self.PlayerInfo`))) (`self.BaseAttackSpeed`) (`BonkItemInteractableComponent.SwingSpeedMultiplier` (`BonkItemInteractComponent.CurrentInteractable` (`self.InteractComp`))))
        (:`then`
          (`GameplayStatics.PlaySoundAtLocation` "/Game/SoundEffects/SwingSword.SwingSword" (`self.K2_GetActorLocation`) (struct) 1.0 1.0 0.0 null null null null))))))

(event `OnDamaged_Event` :!signature `self.OnDamaged`
  (params (NewHealth :type "Float (single-precision)") (DamagedApplied :type "Float (single-precision)") (Bonker :type "BonkBonkerComponent Object Reference") (Player :type "BonkPlayerPawn Object Reference"))
  (bind _hiteffect (`self.HitEffect`))
  ;[1 1 1] Damaged Event
  (`|SpawnActorFromClass` "/Game/Core/Interactable/BP_FloatingNumber.BP_FloatingNumber_C" (`KismetMathLibrary.MakeTransform` (`self.K2_GetActorLocation`) (struct) (3.0 3.0 3.0)) "AlwaysSpawn" "OverrideRootScale" null true (`KismetMathLibrary.Conv_IntToDouble` (`KismetMathLibrary.FTrunc` DamagedApplied)) null)
  (`BonkPlayer.OnHealthUpdated` (`self.PlayerInfo`) (`KismetMathLibrary.FTrunc` NewHealth))
  (`|ExecutionSequence`
    (:`then_0`
      (set `self.LastHitTimer` 0.0))
    (:`then_1`
      (`|ExecutionSequence`
        (:`then_0`
          ;;[1 1 1] Play hit effects
          (`MeshComponent.SetScalarParameterValueOnMaterials` (`self.SkeletalComp`) "HitEffect" 1.0)
          (`KismetSystemLibrary.Delay` 0.2)
          (`MeshComponent.SetScalarParameterValueOnMaterials` (`self.SkeletalComp`) "HitEffect" 0.0))
        (:`then_1`
          (`/Engine/EditorBlueprintResources/StandardMacros.IsValid` _hiteffect
            (:`Is Valid`
              (`ActorComponent.Activate` _hiteffect false))))
        (:`then_2`
          (`self.PlayOnDamageForceFeedback`))
        (:`then_3`
          ;;[1 1 1] Play HitSounds
          (bind _returnvalue (`AddComponent|NODE_AddAudioComponent-0`))
          (message `AudioParameterControllerInterface.SetTriggerParameter` _returnvalue "Hit"))
        (:`then_4`
          (bind _output_get (set `self.HitCounter` (+ 1.0 (`self.HitCounter`) 0.0)))
          (bind _returnvalue_2 (== 4.0 _output_get))
          (if _returnvalue_2
            (bind _returnvalue_3 (`AddComponent|NODE_AddAudioComponent-1`))
            (message `AudioParameterControllerInterface.SetTriggerParameter` _returnvalue_3 "Hit2")))
        (:`then_5`
          (if _returnvalue_2
            (set `self.HitCounter` 0.0)))
        (:`then_6`
          (if (`KismetSystemLibrary.IsValid` Bonker)
            ;;[1 1 1] Hit by Spinner Sound
            (if (== (`GameplayStatics.GetObjectClass` (`ActorComponent.GetOwner` Bonker)) "/Game/WorldInteractions/BP_SpinningSwiper.BP_SpinningSwiper_C")
              (`GameplayStatics.PlaySoundAtLocation` "/Game/SoundEffects/SpinnerHit.SpinnerHit" (`self.K2_GetActorLocation`) (struct) 1.0 1.0 0.0 "/Game/SoundEffects/Attenuation.Attenuation" null null null))
            (else
              (`self.SetRandomBodyRotation`)
              (`KismetSystemLibrary.Delay` 0.2)
              (set `self.TargetBodyRotation` (struct)))))))))

(event `self.ReceiveTick`
  (params (DeltaSeconds :type "Float (single-precision)"))
  (bind _hiteffect (`self.HitEffect`))
  (bind _walkeffect (`self.WalkEffect`))
  (bind _returnvalue (== (`ActorComponent.IsActive` _walkeffect) false))
  ;[1 1 1] Tick
  ;;[1 1 1] Hit Timer
  (`|ExecutionSequence`
    (:`then_0`
      (`self.UpdateLastHitTimer` DeltaSeconds))
    (:`then_1`
      (`self.UpdatePlayerShadow`))
    (:`then_2`
      ;;[1 1 1] Hit FX
      (`KismetSystemLibrary.Delay` 0.1)
      (`/Engine/EditorBlueprintResources/StandardMacros.IsValid` _hiteffect
        (:`Is Valid`
          (if (and (`self.bIsGrounded`) (`ActorComponent.IsActive` _hiteffect))
            (`ActorComponent.Deactivate` _hiteffect)))))
    (:`then_3`
      (`/Engine/EditorBlueprintResources/StandardMacros.IsValid` _walkeffect
        (:`Is Valid`
          (if (> (`KismetMathLibrary.VSize` (`SceneComponent.GetComponentVelocity` (`self.CapsuleComp`))) 100.0)
            (if _returnvalue
              (`ActorComponent.Activate` _walkeffect false))
            (elif (not _returnvalue)
              (`ActorComponent.Deactivate` _walkeffect))))))
    (:`then_4`
      (set `self.BodyRotation` (`KismetMathLibrary.RInterpTo` (`self.BodyRotation`) (`self.TargetBodyRotation`) (`GameplayStatics.GetWorldDeltaSeconds`) 5.0)))
    (:`then_5`
      (`self.LogStats`))
    (:`then_6`
      (`self.BountyUI`))))

(event `self.BonkableComp.OnHitResponse`
  (params (BonkerComponent :type "BonkBonkerComponent Object Reference") (Hit :type "HitResult Structure"))
  (set `self.GroundTraceLength` 0.0)
  (`self.SetHitRotation` Hit 45.0)
  (`KismetSystemLibrary.Delay` 0.2)
  (set `self.GroundTraceLength` 20.0)
  (set `self.TargetBodyRotation` (struct)))

(event `OnBonkerHit_Event` :!signature `self.OnBonkerHit`
  (params (Actor :type "Actor Object Reference"))
  (`BonkAbilityComponent.OnHit` (`self.AbilityComp`) Actor)
  (bind _aswbp_bounty_player (cast `/Game/Widgets/WBP_BountyPlayer` (`WidgetComponent.GetUserWidgetObject` (`self.Widget`))))
  (`/Game/Widgets/WBP_BountyPlayer.ShakeAnim` _aswbp_bounty_player))

(event `self.InteractComp.OnStartThrow`
  (`GameplayStatics.PlaySoundAtLocation` "/Game/SoundEffects/ThrowStart.ThrowStart" (`self.K2_GetActorLocation`) (struct) 0.5 1.0 0.0 null null null null)
  (`KismetSystemLibrary.PrintString` "THROW"))

(event `PlayHitForceFeedBack`
  (params (Actor :type "Actor Object Reference"))
  (if (== (`GameplayStatics.GetObjectClass` Actor) "BP_BonkPlayerPawn_C")
    (`PlayerController.K2_ClientPlayForceFeedback` (`GameplayStatics.GetPlayerController` (`BonkPlayer.PlayerIndex` (`self.PlayerInfo`))) "/Game/Player/ForceFeedbacks/FF_OnHit.FF_OnHit" "None" false false false)))

(event `self.InteractComp.OnDrop`
  (params (Interactable :type "BonkItemInteractableComponent Object Reference"))
  (`GameplayStatics.PlaySoundAtLocation` "/Game/SoundEffects/ThrowRelease.ThrowRelease" (`self.K2_GetActorLocation`) (struct) 1.5 1.0 0.0 null null null null)
  (`BonkAbilityComponent.OnDrop` (`self.AbilityComp`) (`ActorComponent.GetOwner` Interactable)))

(event `PlayOnDamageForceFeedback`
  (`PlayerController.K2_ClientPlayForceFeedback` (`GameplayStatics.GetPlayerController` (`BonkPlayer.PlayerIndex` (`self.PlayerInfo`))) "/Game/Player/ForceFeedbacks/FF_OnDamage.FF_OnDamage" "None" false false false))

(event `self.InteractComp.OnPickup`
  (params (Interactable :type "BonkItemInteractableComponent Object Reference"))
  (`GameplayStatics.PlaySoundAtLocation` "/Game/SoundEffects/Pickup_weapon.Pickup_weapon" (`self.K2_GetActorLocation`) (struct) 0.5 1.0 0.0 "/Game/SoundEffects/Attenuation.Attenuation" null null null)
  (`|PlayMontage` (`self.SkeletalComp`) "/Game/Animation/AM_Pickup.AM_Pickup" 1.0 0.1))

(event `PlayDeathForceFeedback`
  (`PlayerController.K2_ClientPlayForceFeedback` (`GameplayStatics.GetPlayerController` (`BonkPlayer.PlayerIndex` (`self.PlayerInfo`))) "/Game/Player/ForceFeedbacks/FF_OnDeath.FF_OnDeath" "None" false false false))

(event `OnHealed_Event` :!signature `self.OnHealed`
  (params (NewHealth :type "Float (single-precision)") (HealthApplied :type "Float (single-precision)"))
  (`|SpawnActorFromClass` "/Game/Core/Interactable/BP_FloatingNumber.BP_FloatingNumber_C" (`KismetMathLibrary.MakeTransform` (`self.K2_GetActorLocation`) (struct) (1.8 1.8 1.8)) "AlwaysSpawn" "OverrideRootScale" null false (`KismetMathLibrary.Conv_IntToDouble` (`KismetMathLibrary.FTrunc` HealthApplied)) null))

(event `OnKilll_Event`
  (params (NewKillCount :type Integer))
  (`SceneComponent.SetVisibility` (`self.Widget`) true false)
  (bind _aswbp_bounty_player (cast `/Game/Widgets/WBP_BountyPlayer` (`WidgetComponent.GetUserWidgetObject` (`self.Widget`))))
  (`/Game/Widgets/WBP_BountyPlayer.ShakeAnim` _aswbp_bounty_player))

(fn `Bonk`
  (`BonkBonkableComponent.KnockbackFromDirection` (`self.BonkableComp`) (* (`KismetMathLibrary.Vector_Forward`) 2000.0) 0.0))

(fn `BountyUI`
  (bind _cameraref (`self.CameraRef`)
    (:`then`
      (bind (_returnvalue_roll _returnvalue_pitch _returnvalue_yaw) (`KismetMathLibrary.BreakRotator` (`KismetMathLibrary.FindLookAtRotation` (`SceneComponent.K2_GetComponentLocation` (`self.Widget`)) (`self.K2_GetActorLocation` _cameraref))))
      (`SceneComponent.K2_SetWorldRotation` (`self.Widget`) (`KismetMathLibrary.MakeRotator` 0.0 0.0 _returnvalue_yaw) false false))
    (:`else`)))

(fn `CreateVFX`
  (bind _skeletalcomp (`self.SkeletalComp`))
  (`|ExecutionSequence`
    (:`then_0`
      (bind _returnvalue (`NiagaraFunctionLibrary.SpawnSystemAttached` "/Game/Art/VFX/sA_StylizedMix/Fx/NS_RunningDust.NS_RunningDust" _skeletalcomp "None" (0.0 0.0 0.0) (struct :`Yaw` 90.0) "KeepRelativeOffset"))
      (set `self.WalkEffect` _returnvalue))
    (:`then_1`
      (bind _returnvalue_2 (`NiagaraFunctionLibrary.SpawnSystemAttached` "/Game/Art/VFX/sA_StylizedMix/Fx/NS_Smoke_White.NS_Smoke_White" _skeletalcomp "None" (0.0 0.0 0.0) (struct) "KeepRelativeOffset"))
      (set `self.HitEffect` _returnvalue_2))
    (:`then_2`
      (bind _returnvalue_3 (`NiagaraFunctionLibrary.SpawnSystemAttached` "/Game/Art/VFX/sA_StylizedMix/Fx/NS_Smokeless_Flame_1.NS_Smokeless_Flame_1" (`self.SkeletalComp`) "None" (0.0 0.0 0.0) (struct) "KeepRelativeOffset" false false))
      (bind _output_get (set `self.FireEffect` _returnvalue_3))
      (`SceneComponent.SetRelativeScale3D` _output_get (0.3 0.3 0.3)))))

(fn `KillPlayer`
  (locals (GameModeRef :type "BonkGameModeBase Object Reference"))
  (bind _returnvalue (`BonkGameModeBase.Get`))
  (bind _lasthittimer (`self.LastHitTimer`))
  (bind _playerindex (`BonkPlayer.PlayerIndex` (`self.PlayerInfo`)))
  (bind _playerindex_2 (`BonkPlayer.PlayerIndex` (`self.PlayerInfo`)))
  (`/Engine/EditorBlueprintResources/StandardMacros.IsValid` _returnvalue
    (:`Is Valid`
      (set `local.GameModeRef` _returnvalue))
    (:`Is Not Valid`
      _))
  (if (and (<= _lasthittimer 10.0) (!= _lasthittimer -1.0))
    ;[1 1 1] Been hit
    (`BonkBonkableComponent.LastBonkerHit` (`self.BonkableComp`)
      (:`then`
        ;[1 1 1] Last damage by this bonker
        (bind _lastdamagedby (`self.LastDamagedBy`)
          (:`then`
            (bind _asbp_weap_base (cast `/Game/Core/Interactable/Weapons/BP_Weap_Base` (`ActorComponent.GetOwner` _lastdamagedby))
              (:`then`
                ;[1 1 1] Player that last owned bonker
                (bind _asbp_bonk_player_pawn (cast `/Game/Player/BP_BonkPlayerPawn` (`ActorComponent.GetOwner` (`BonkItemInteractableComponent.LastHeldByInteract` (`BonkBonker.InteractableComponent` _asbp_weap_base))))
                  (:`then`
                    ;[1 1 1] Killed by Player
                    (bind _gamemoderef (`local.GameModeRef`)
                      (:`then`
                        (bind _playerindex_3 (`BonkPlayer.PlayerIndex` (`BonkPlayerPawn.PlayerInfo` _asbp_bonk_player_pawn)))
                        (`BonkGameModeBase.PlayerDied` _gamemoderef _playerindex _playerindex_3))
                      (:`else`
                        _))
                    (`KismetSystemLibrary.PrintString` (`KismetStringLibrary.Concat_StrStr` (`KismetStringLibrary.Conv_IntToString` _playerindex_3) " killed " (`KismetStringLibrary.Conv_IntToString` _playerindex))))
                  (:`CastFailed`
                    ;[1 1 1] Not killed by player
                    (bind _gamemoderef_2 (`local.GameModeRef` :!label _label)
                      (:`then`
                        (`BonkGameModeBase.PlayerDied` _gamemoderef_2 _playerindex_2 -1))
                      (:`else`
                        _))
                    (`KismetSystemLibrary.PrintString` (`KismetStringLibrary.Concat_StrStr` "Suicide" " killed " (`KismetStringLibrary.Conv_IntToString` _playerindex_2))))))
              (:`CastFailed`
                (goto _label))))
          (:`else`)))
      (:`else`
        (goto _label)))
    (else
      (goto _label))))

(fn `LogStats`
  (bind _playerinfo (`self.PlayerInfo`))
  (if (`self.DebugLog`)
    (`KismetSystemLibrary.PrintString` "-------------------" true true (struct :`R` 1.0 :`G` 1.0 :`B` 1.0 :`A` 1.0) 0.0)
    (`KismetSystemLibrary.PrintString` (`KismetStringLibrary.Concat_StrStr` "KillCount: " (`KismetStringLibrary.Conv_IntToString` (`BonkPlayer.KillCount` _playerinfo))) true true (struct :`R` 1.0 :`A` 1.0) 0.0)
    (`KismetSystemLibrary.PrintString` (`KismetStringLibrary.Concat_StrStr` "BountyCount: " (`KismetStringLibrary.Conv_IntToString` (`BonkPlayer.BountyCount` _playerinfo))) true true (struct :`R` 1.0 :`A` 1.0) 0.0)
    (`KismetSystemLibrary.PrintString` (`KismetStringLibrary.Concat_StrStr` "AttackSpeed: " (`KismetStringLibrary.Conv_DoubleToString` (`BonkAttribute.CurrentValue` (`BonkPlayer.AttackSpeed` _playerinfo)))) true true (struct :`R` 1.0 :`G` 1.0 :`B` 1.0 :`A` 1.0) 0.0)
    (`KismetSystemLibrary.PrintString` (`KismetStringLibrary.Concat_StrStr` "MoveSpeed: " (`KismetStringLibrary.Conv_DoubleToString` (`BonkAttribute.CurrentValue` (`BonkPlayer.MoveSpeed` _playerinfo)))) true true (struct :`R` 1.0 :`G` 1.0 :`B` 1.0 :`A` 1.0) 0.0)
    (`KismetSystemLibrary.PrintString` (`KismetStringLibrary.Concat_StrStr` "Health: " (`KismetStringLibrary.Conv_DoubleToString` (`BonkAttribute.CurrentValue` (`BonkPlayer.Health` _playerinfo)))) true true (struct :`R` 1.0 :`G` 1.0 :`B` 1.0 :`A` 1.0) 0.0)
    (`KismetSystemLibrary.PrintString` (`KismetStringLibrary.Concat_StrStr` "Damage: " (`KismetStringLibrary.Conv_DoubleToString` (`BonkAttribute.CurrentValue` (`BonkPlayer.Damage` _playerinfo)))) true true (struct :`R` 1.0 :`G` 1.0 :`B` 1.0 :`A` 1.0) 0.0)
    (`KismetSystemLibrary.PrintString` (`KismetStringLibrary.Concat_StrStr` "Resilience: " (`KismetStringLibrary.Conv_DoubleToString` (`BonkAttribute.CurrentValue` (`BonkPlayer.Resilience` _playerinfo)))) true true (struct :`R` 1.0 :`G` 1.0 :`B` 1.0 :`A` 1.0) 0.0)
    (`KismetSystemLibrary.PrintString` (`KismetStringLibrary.Concat_StrStr` "WeaponSize: " (`KismetStringLibrary.Conv_DoubleToString` (`BonkAttribute.CurrentValue` (`BonkPlayer.WeaponSize` _playerinfo)))) true true (struct :`R` 1.0 :`G` 1.0 :`B` 1.0 :`A` 1.0) 0.0)
    (`KismetSystemLibrary.PrintString` (`KismetStringLibrary.Concat_StrStr` "Player " (`KismetStringLibrary.Conv_IntToString` (`BonkPlayer.PlayerIndex` (`self.PlayerInfo`)))) true true (struct :`G` 0.66 :`B` 1.0 :`A` 1.0) 0.0)
    (`KismetSystemLibrary.PrintString` "-------------------" true true (struct :`R` 1.0 :`G` 1.0 :`B` 1.0 :`A` 1.0) 0.0)))

(fn `SetHitRotation`
  (params (Hit :type "HitResult Structure (by ref)") (Rotation :type "Float (double-precision)"))
  (bind _returnvalue (`self.K2_GetActorLocation`))
  (bind _returnvalue_2 (`self.K2_GetActorLocation`))
  (bind _returnvalue_3 (`self.K2_GetActorLocation`))
  (bind _returnvalue_4 (`self.K2_GetActorLocation`))
  (bind (_returnvalue_x _returnvalue_y) (`KismetMathLibrary.BreakVector` (+ _returnvalue_3 (* (0.0 0.0 0.0) 50.0))))
  (bind (_returnvalue_x_2 _returnvalue_y_2) (`KismetMathLibrary.BreakVector` (- (`.ImpactPoint` (`GameplayStatics.BreakHitResult` Hit)) (`self.K2_GetActorLocation`))))
  (bind _returnvalue_5 (`KismetMathLibrary.Normal` (`KismetMathLibrary.MakeVector` _returnvalue_x_2 _returnvalue_y_2)))
  (bind _returnvalue_6 (`KismetMathLibrary.RotateAngleAxis` _returnvalue_5 -90.0 (0.0 0.0 1.0)))
  (bind (_returnvalue_x_3 _returnvalue_y_3) (`KismetMathLibrary.BreakVector` (+ _returnvalue (* _returnvalue_5 50.0))))
  (bind (_returnvalue_x_4 _returnvalue_y_4) (`KismetMathLibrary.BreakVector` (+ _returnvalue_4 (* _returnvalue_6 50.0))))
  (`KismetSystemLibrary.DrawDebugLine` _returnvalue (`KismetMathLibrary.MakeVector` _returnvalue_x_3 _returnvalue_y_3 (.z _returnvalue)) (struct :`R` 1.0 :`A` 1.0) 2.0 3.0)
  (`KismetSystemLibrary.DrawDebugLine` _returnvalue_4 (`KismetMathLibrary.MakeVector` _returnvalue_x_4 _returnvalue_y_4 (.z _returnvalue_4)) (struct :`G` 1.0 :`A` 1.0) 2.0 3.0)
  (`KismetSystemLibrary.DrawDebugLine` _returnvalue_2 (+ _returnvalue_2 (* (`KismetMathLibrary.Vector_Up`) 50.0)) (struct :`B` 1.0 :`A` 1.0) 2.0 3.0)
  (`KismetSystemLibrary.DrawDebugLine` _returnvalue_3 (`KismetMathLibrary.MakeVector` _returnvalue_x _returnvalue_y (.z _returnvalue_3)) (struct :`R` 1.0 :`G` 1.0 :`A` 1.0) 2.0 3.0)
  (set `self.TargetBodyRotation` (`KismetMathLibrary.RotatorFromAxisAndAngle` _returnvalue_6 Rotation)))

(fn `SetPawnColors`
  (bind (_returnvalue_teamname _returnvalue_teamcolor) (break `TeamStructure` (`BonkGameModeBase.GetTeam` (`BonkGameModeBase.Get`) (`BonkPlayer.TeamIndex` (`self.PlayerInfo`)))))
  (bind (_returnvalue_teamname_2 _returnvalue_teamcolor_2) (break `TeamStructure` (`BonkGameModeBase.GetTeam` (`BonkGameModeBase.Get`) (`BonkPlayer.TeamIndex` (`self.PlayerInfo`)))))
  (`/Engine/EditorBlueprintResources/StandardMacros.IsValid` (`BonkGameModeBase.Get`)
    (:`Is Valid`
      (`|ExecutionSequence`
        (:`then_0`
          ;[1 1 1] Set pawn to team color (prototype)
          (bind _returnvalue (`PrimitiveComponent.CreateDynamicMaterialInstance` (`self.SkeletalComp`) 0 "/Game/Art/Materials/Prototyping/M_SingleColor.M_SingleColor" "None"))
          (`MaterialInstanceDynamic.SetVectorParameterValue` _returnvalue "Color" (`KismetMathLibrary.Conv_ColorToLinearColor` _returnvalue_teamcolor_2)))
        (:`then_1`
          (bind _returnvalue_2 (`DecalComponent.CreateDynamicMaterialInstance` (`self.Decal`)))
          (`MaterialInstanceDynamic.SetVectorParameterValue` _returnvalue_2 "Color" (`KismetMathLibrary.Conv_ColorToLinearColor` _returnvalue_teamcolor)))))))

(fn `SetPlayerData`
  (if (`self.Debug`)
    (bind _returnvalue (`|GenericCreateObject` "/Script/Bonk.BonkPlayer"))
    (bind _output_get (set `self.PlayerInfo` _returnvalue))
    (`BonkAbilityComponent.SetPlayerData` (`self.AbilityComp`) _output_get)
    ;[1 1 1] Health reset
    (`BonkAttribute.SetCurrentValue` (`BonkPlayer.Health` (`self.PlayerInfo`)) 0.0)
    (else
      (bind _playerinfo (`self.PlayerInfo`)
        (:`then`
          (`BonkAbilityComponent.SetPlayerData` (`self.AbilityComp`) _playerinfo)
          (`BonkAttribute.SetCurrentValue` (`BonkPlayer.Health` (`self.PlayerInfo`)) 0.0))
        (:`else`)))))

(fn `SetRandomBodyRotation`
  (locals (RandomRoll :type "Float (double-precision)") (RandomPitch :type "Float (double-precision)"))
  (bind _output_get (set `local.RandomRoll` (* (`KismetMathLibrary.RandomFloatInRange` 10.0 25.0) (`|GetArrayItem` (`self.UnitArray`) (`KismetMathLibrary.RandomIntegerInRange` 0 1)))))
  (bind _output_get_2 (set `local.RandomPitch` (* (`KismetMathLibrary.RandomFloatInRange` 10.0 25.0) (`|GetArrayItem` (`self.UnitArray`) (`KismetMathLibrary.RandomIntegerInRange` 0 1)))))
  (set `self.TargetBodyRotation` (`KismetMathLibrary.MakeRotator` _output_get _output_get_2)))

(fn `UpdateLastHitTimer`
  (params (`Delta time` :type "Float (double-precision)"))
  (if (!= (`self.LastHitTimer`) -1.0)
    (set `self.LastHitTimer` (+ `Delta time` (`self.LastHitTimer`)))))

(fn `UpdatePlayerShadow`
  (bind (_outhit _returnvalue) (`KismetSystemLibrary.LineTraceSingle` :`Start` (`self.K2_GetActorLocation`) :`End` (+ (`self.K2_GetActorLocation`) (* (`self.GetActorUpVector`) -100000.0)) :`TraceChannel` "TraceTypeQuery3" :`DrawDebugType` "ForOneFrame" :`TraceColor` (struct :`G` 1.0 :`B` 0.99254 :`A` 1.0) :`TraceHitColor` (struct :`R` 0.984814 :`G` 1.0 :`A` 1.0)))
  (if _returnvalue
    (bind (_bblockinghit _binitialoverlap _time _distance _location _impactpoint _normal _impactnormal) (`GameplayStatics.BreakHitResult` _outhit))
    (`SceneComponent.K2_SetWorldTransform` (`self.Decal`) (`KismetMathLibrary.MakeTransform` _impactpoint (`KismetMathLibrary.Conv_VectorToRotator` _impactnormal)) false false)
    (`SceneComponent.SetRelativeScale3D` (`self.Decal`) (/ (`KismetMathLibrary.VLerp` (50.0 50.0 50.0) (20.0 20.0 20.0) (`KismetMathLibrary.FClamp` (/ _distance 500.0))) 50.0))))

(fn `UserConstructionScript`)