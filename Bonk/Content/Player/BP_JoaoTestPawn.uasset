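; Test player pawn with camera-relative movement on a physics capsule, registering a new BonkPlayer with its ability component on BeginPlay.
; Each tick projects input onto BP_JoaoTestCamera's flattened axes and interpolates toward a goal velocity using ground or air tuning, overwriting the capsule's entire linear velocity.
; A downward sphere trace then updates grounded state, and yaw eases toward input.
; Debug prints and lines run every frame; deceleration and dot-scaled acceleration are computed but unused.
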(event `InputAction|Jump`
  (params (Key :type "Key Structure")))

(event `InputAxis|Move Right/Left`
  (params (AxisValue :type "Float (single-precision)"))
  (set `self.InputMoveRight` AxisValue))

(event `InputAxis|Move Forward/Backward`
  (params (AxisValue :type "Float (single-precision)"))
  (set `self.InputMoveForward` AxisValue))

(event `self.ReceiveBeginPlay`
  (`self.Init`))

(event `self.ReceiveTick`
  (params (DeltaSeconds :type "Float (single-precision)"))
  (`|ExecutionSequence`
    (:`then_0`
      (`self.Debug`))
    (:`then_1`
      (`self.ExecuteMovement`))
    (:`then_2`
      (`self.GroundCheck`))
    (:`then_3`
      (`self.ExecuteRotation`))))

(fn `Debug`
  (bind _returnvalue (`self.K2_GetActorLocation`))
  (bind _returnvalue_2 (`self.K2_GetActorLocation`))
  (bind _returnvalue_3 (`self.K2_GetActorLocation`))
  (`|ExecutionSequence`
    (:`then_0`
      (`KismetSystemLibrary.PrintString` (`KismetStringLibrary.Concat_StrStr` "Move: " (`KismetStringLibrary.Conv_VectorToString` (`self.InputMove`))) true true (struct :`R` 1.0 :`G` 1.0 :`B` 1.0 :`A` 1.0) 0.0)
      (`KismetSystemLibrary.PrintString` (`KismetStringLibrary.Concat_StrStr` "GroundVelocity: " (`KismetStringLibrary.Conv_VectorToString` (`self.GroundVelocity`))) true true (struct :`R` 1.0 :`G` 1.0 :`B` 1.0 :`A` 1.0) 0.0)
      (`KismetSystemLibrary.PrintString` (`KismetStringLibrary.Concat_StrStr` "GroundVelocity: " (`KismetStringLibrary.Conv_VectorToString` (`SceneComponent.GetComponentVelocity` (`self.Capsule`)))) true true (struct :`R` 1.0 :`G` 1.0 :`B` 1.0 :`A` 1.0) 0.0)
      (`KismetSystemLibrary.PrintString` (`KismetStringLibrary.Concat_StrStr` "InputVelocityDot: " (`KismetStringLibrary.Conv_DoubleToString` (`self.InputVelocityDot`))) true true (struct :`R` 1.0 :`G` 1.0 :`B` 1.0 :`A` 1.0) 0.0))
    (:`then_1`
      (`KismetSystemLibrary.DrawDebugLine` _returnvalue (+ _returnvalue (* (`self.InputMoveUnit`) 150.0)) (struct :`R` 1.0 :`A` 1.0) 0.0 5.0)
      (`KismetSystemLibrary.DrawDebugLine` _returnvalue_2 (+ _returnvalue_2 (* (`KismetMathLibrary.Normal` (`self.GroundVelocity`)) 150.0)) (struct :`B` 1.0 :`A` 1.0) 0.0 5.0)
      (`KismetSystemLibrary.DrawDebugLine` _returnvalue_3 (+ _returnvalue_3 (* (`KismetMathLibrary.Normal` (`SceneComponent.GetComponentVelocity` (`self.Capsule`))) 150.0)) (struct :`R` 1.0 :`G` 0.536849 :`A` 1.0) 0.0 5.0))))

(fn `ExecuteMovement`
  (locals (Accel :type "Float (double-precision)") (Speed :type "Float (double-precision)") (Deaccel :type "Float (double-precision)") (FinalAccel :type "Float (double-precision)") (GoalVelocity :type "Vector Structure"))
  (bind _cameraactor (`self.CameraActor`))
  (bind (_returnvalue_x _returnvalue_y) (`KismetMathLibrary.BreakVector` (`SceneComponent.GetComponentVelocity` (`self.Capsule`))))
  ;[1 1 1] Input Movement (relative to camera)
  (bind _output_get (set `self.InputMove` (+ (* (`KismetMathLibrary.ProjectVectorOnToPlane` (`self.GetActorRightVector` _cameraactor) (0.0 0.0 1.0)) (`self.InputMoveRight`)) (* (`KismetMathLibrary.ProjectVectorOnToPlane` (`self.GetActorForwardVector` _cameraactor) (0.0 0.0 1.0)) (`self.InputMoveForward`)))))
  ;[1 1 1] Capping input move at 1
  (if (> (`KismetMathLibrary.VSize` _output_get) 1.0)
    (set `self.InputMoveUnit` (`KismetMathLibrary.Normal` (`self.InputMove`)))
    (else
      (set `self.InputMoveUnit` (`self.InputMove`))))
  ;[1 1 1] Ground velocity (z = 0)
  (set `self.GroundVelocity` (`KismetMathLibrary.MakeVector` _returnvalue_x _returnvalue_y))
  (set `self.InputVelocityDot` (`KismetMathLibrary.Dot_VectorVector` (`KismetMathLibrary.Normal` (`self.GroundVelocity`)) (`KismetMathLibrary.Normal` (`self.InputMove`))))
  (if (`self.IsGrounded`)
    (set `local.Accel` (`self.GroundAccel`))
    (set `local.Deaccel` (`self.GroundDeaccel`))
    (set `local.Speed` (`self.GroundSpeed`))
    (else
      (set `local.Accel` (`self.AirAccel`))
      (set `local.Deaccel` (`self.AirDeaccel`))
      (set `local.Speed` (* (`self.GroundSpeed`) (`self.AirControl`)))))
  (set `local.FinalAccel` (* (`local.Accel`) (`self.InputVelocityDot`)))
  (set `local.GoalVelocity` (* (`self.InputMoveUnit`) (`local.Speed`)))
  (bind _output_get_2 (set `self.CurrentVelocity` (`KismetMathLibrary.VInterpTo` (`self.CurrentVelocity`) (`local.GoalVelocity`) (`GameplayStatics.GetWorldDeltaSeconds`) (`local.Accel`))))
  (`PrimitiveComponent.SetPhysicsLinearVelocity` (`self.Capsule`) _output_get_2 false "None"))

(fn `ExecuteRotation`
  (bind (_returnvalue_roll _returnvalue_pitch) (`KismetMathLibrary.BreakRotator` (`self.K2_GetActorRotation`)))
  (bind _inputmove (`self.InputMove`))
  (bind (_returnvalue_roll_2 _returnvalue_pitch_2 _returnvalue_yaw) (`KismetMathLibrary.BreakRotator` (`KismetMathLibrary.RInterpTo` (`self.CurrentRotation`) (`KismetMathLibrary.FindLookAtRotation` (`KismetMathLibrary.Vector_Zero`) (`self.RotationDirection`)) (`GameplayStatics.GetWorldDeltaSeconds`) (`self.RotationSpeed`))))
  (if (> (`KismetMathLibrary.VSize` _inputmove) 0.5)
    (set `self.RotationDirection` _inputmove)
    ;[1 1 1] Rotation
    (bind _output_get (set `self.CurrentRotation` (`KismetMathLibrary.MakeRotator` 0.0 0.0 _returnvalue_yaw)))
    (`self.K2_SetActorRotation` (`KismetMathLibrary.MakeRotator` _returnvalue_roll _returnvalue_pitch (.yaw _output_get)))))

(fn `GroundCheck`
  (locals (TraceVelDot :type "Float (double-precision)") (RideOffset :type "Float (double-precision)"))
  (bind _returnvalue (`self.K2_GetActorLocation`))
  (bind _outhit (`KismetSystemLibrary.SphereTraceSingle` :`Start` _returnvalue :`End` (- _returnvalue (* (`self.GetActorUpVector`) (`self.RideTraceLength`))) :`Radius` (`self.GroundTraceRadius`) :`TraceChannel` "TraceTypeQuery3" :`DrawDebugType` "ForOneFrame"))
  (bind (_bblockinghit _binitialoverlap _time _distance _location _impactpoint _normal _impactnormal _physmat _hitactor _hitcomponent _hitbonename _bonename _hititem _elementindex _faceindex _tracestart) (`GameplayStatics.BreakHitResult` _outhit))
  (if _bblockinghit
    (set `self.IsGrounded` true)
    (set `self.GroundNormal` _impactnormal)
    (else
      (set `self.IsGrounded` false)
      (set `self.GroundNormal` _impactnormal))))

(fn `Init`
  (bind _returnvalue (`|GenericCreateObject` "/Script/Bonk.BonkPlayer"))
  (bind _output_get (set `self.PlayerInfo` _returnvalue))
  (`BonkAbilityComponent.SetPlayerData` (`self.BonkAbilityComponent`) _output_get)
  (bind _returnvalue_2 (`GameplayStatics.GetActorOfClass` "/Game/Player/BP_JoaoTestCamera.BP_JoaoTestCamera_C"))
  (set `self.CameraActor` _returnvalue_2))

(fn `UserConstructionScript`)