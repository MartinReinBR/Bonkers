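; BP_JoaoTestCamera is a test follow camera that frames a group of target actors and takes over player 0's view at BeginPlay.
; Each tick it averages the target actors' locations, adds an offset along a direction vector, and smoothly interpolates itself toward that point.
; It also reapplies a configurable pitch to its camera component's relative rotation every frame.
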(event `self.ReceiveBeginPlay`
  (set `self.bFindCameraComponentWhenViewTarget` true)
  (`PlayerController.SetViewTargetWithBlend` (`GameplayStatics.GetPlayerController` 0) self 0.0 "VTBlend_Linear" 0.0 false))

(event `self.ReceiveTick`
  (params (DeltaSeconds :type "Float (single-precision)"))
  (bind _returnvalue (`GameplayStatics.GetActorArrayAverageLocation` (`self.TargetActors`)))
  (`self.K2_SetActorLocation` (`KismetMathLibrary.VInterpTo` (`self.K2_GetActorLocation`) (+ _returnvalue (* (`self.Direction`) (`self.Offset`))) DeltaSeconds (`self.InterpSpeed`)))
  (`SceneComponent.K2_SetRelativeRotation` (`self.Camera`) (`KismetMathLibrary.MakeRotator` 0.0 (`self.Pitch`)) false false))

(fn `UserConstructionScript`)