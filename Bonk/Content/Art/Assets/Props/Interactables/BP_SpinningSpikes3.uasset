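; Spinning spikes prop that rotates a physics mesh constantly and speeds up when activated.
; Tick drives the mesh's Z angular velocity to a target speed, which activation multiplies from the default.
; Deactivation starts a timer to restore normal speed after a delay, and reactivation cancels any pending timer.
; A BonkBonkerSphere component traces between two scene points from BeginPlay, though its hit event is empty here.
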(event `self.ReceiveBeginPlay`
  (bind _bonkbonkersphere (`self.BonkBonkerSphere`))
  (`PrimitiveComponent.WakeRigidBody` (`self.StaticMesh`) "None")
  (set `self.TargetSpinSpeed` (`self.DefaultSpinSpeed`))
  (`BonkBonkerComponent.ActivateTracing` _bonkbonkersphere true)
  (`BonkBonkerComponent.SetTraceLocationFromSceneComps` _bonkbonkersphere (`self.TraceStart`) (`self.TraceEnd`)))

(event `self.ReceiveTick`
  (params (DeltaSeconds :type "Float (single-precision)"))
  (`PrimitiveComponent.SetPhysicsAngularVelocityInDegrees` (`self.StaticMesh`) (`KismetMathLibrary.MakeVector` 0.0 0.0 (`self.TargetSpinSpeed`)) false "None"))

(event `/Game/WorldInteractions/BI_ToggleableInterface.OnActivate`
  (bind _deactivateevent (`self.DeactivateEvent`))
  (`|ExecutionSequence`
    (:`then_0`
      (if (`KismetSystemLibrary.K2_IsValidTimerHandle` _deactivateevent)
        (`KismetSystemLibrary.K2_ClearAndInvalidateTimerHandle` _deactivateevent)))
    (:`then_1`
      (set `self.TargetSpinSpeed` (* (`self.DefaultSpinSpeed`) (`self.SpinSpeedMultiplier`))))))

(event `/Game/WorldInteractions/BI_ToggleableInterface.OnDeactivate`
  (if (not (`KismetSystemLibrary.K2_IsValidTimerHandle` (`self.DeactivateEvent`)))
    (bind _returnvalue (`KismetSystemLibrary.K2_SetTimerDelegate` (`|CreateDelegate` :!event `DeactivateOnTimer`) (`self.BackToNormalSpinTime`)))
    (set `self.DeactivateEvent` _returnvalue)))

(event `DeactivateOnTimer`
  (set `self.TargetSpinSpeed` (`self.DefaultSpinSpeed`)))

(event `self.BonkBonkerSphere.OnHit`
  (params (BonkableComponent :type "BonkBonkableComponent Object Reference") (FHitResult :type "HitResult Structure")))

(fn `UserConstructionScript`)