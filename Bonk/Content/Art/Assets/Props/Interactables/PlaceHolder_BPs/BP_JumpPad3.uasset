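; BP_JumpPad3 is a placeholder jump pad that launches the player pawn along the world left vector.
; When a BP_BonkPlayerPawn overlaps the Box, its capsule receives a mass-independent velocity-change impulse scaled by ImpulseForce.
; It also plays an attenuated bounce sound and restarts a timeline that scales the static mesh relative to its world scale cached at BeginPlay.
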(event `self.ReceiveBeginPlay`
  (set `self.Relative Scale` (`SceneComponent.K2_GetComponentScale` (`self.StaticMesh`))))

(event `self.Box.OnComponentBeginOverlap`
  (params (OverlappedComponent :type "PrimitiveComponent Object Reference") (OtherActor :type "Actor Object Reference") (OtherComp :type "PrimitiveComponent Object Reference") (OtherBodyIndex :type Integer) (bFromSweep :type Boolean) (SweepResult :type "HitResult Structure (by ref)"))
  (bind _asbp_bonk_player_pawn (cast `/Game/Player/BP_BonkPlayerPawn` OtherActor))
  (`PrimitiveComponent.AddImpulse` (`BonkPlayerPawn.CapsuleComp` _asbp_bonk_player_pawn) (* (`KismetMathLibrary.Vector_Left`) (`self.ImpulseForce`)) "None" true)
  (`GameplayStatics.PlaySoundAtLocation` "/Game/SoundEffects/Bounce.Bounce" (`self.K2_GetActorLocation`) (struct) 1.0 1.0 0.0 "/Game/SoundEffects/Attenuation.Attenuation" null null null)
  (bind (_direction _size) (`Timeline|Timeline_0` :!via `PlayFromStart`)
    (:`Update`
      (`SceneComponent.SetWorldScale3D` (`self.StaticMesh`) (* (`self.Relative Scale`) _size)))))

(fn `UserConstructionScript`)