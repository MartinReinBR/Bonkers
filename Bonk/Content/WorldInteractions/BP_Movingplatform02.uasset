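; Moving platform actor that slides its static mesh toward a configurable EndLoc offset.
; A timeline starts on BeginPlay and drives a linear ease of the mesh's relative location, without sweeping.
; The construction script previews the destination with a temporary debug box sized to the mesh bounds, offset by EndLoc.
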(event `self.ReceiveBeginPlay`
  (bind (_direction _newtrack_0) (`Timeline|Timeline_0`)
    (:`Update`
      (`SceneComponent.K2_SetRelativeLocation` (`self.StaticMesh`) (`|EaseFunction` "Linear" _newtrack_0 (0.0 0.0 0.0) (`self.End_Loc`)) false false))))

(fn `UserConstructionScript`
  (bind (_origin _boxextent) (`KismetSystemLibrary.GetComponentBounds` (`self.StaticMesh`)))
  (`KismetSystemLibrary.DrawDebugBox` (+ (`self.End_Loc`) _origin) _boxextent (struct) (struct) 5.0 10.0))