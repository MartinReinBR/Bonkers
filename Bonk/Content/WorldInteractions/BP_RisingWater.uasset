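; Rising water hazard that splashes when a bonkable actor leaves its overlap and destroys player pawns that exit below its origin height.
; Round start schedules a timer unless button-controlled, where activation starts raising directly; round end or deactivation snaps it back.
; Tick moves it vertically at speed derived from target height and raise time; lowering stops at the initial height.
; Construction script draws a debug plane at the target height.
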(event `self.ReceiveBeginPlay`
  (bind _returnvalue (`BonkGameModeBase.Get`))
  (set `self.InitialLocation` (`self.K2_GetActorLocation`))
  (`/Engine/EditorBlueprintResources/StandardMacros.IsValid` _returnvalue
    (:`Is Valid`
      (if (not (`self.bIsControlledByButton`))
        (add `BonkGameModeBase.OnRoundStart` _returnvalue (`|CreateDelegate` :!event `OnRoundStart_Event_0`)))
      (add `BonkGameModeBase.OnRoundEnd` _returnvalue (`|CreateDelegate` :!event `OnRoundEnd_Event_0`)))))

(event `self.OnActivate`
  (if (`self.bIsControlledByButton`)
    (`self.StartRaising`)))

(event `self.OnDeactivate`
  (`self.SetActorTickEnabled` false)
  (`self.K2_SetActorLocation` (`self.InitialLocation`)))

(event `self.ReceiveTick`
  (params (DeltaSeconds :type "Float (single-precision)"))
  (bind (_returnvalue_x _returnvalue_y _returnvalue_z) (`KismetMathLibrary.BreakVector` (`self.K2_GetActorLocation`)))
  (bind (_initiallocation_x _initiallocation_y _initiallocation_z) (`KismetMathLibrary.BreakVector` (`self.InitialLocation`)))
  (`self.K2_AddActorWorldOffset` (* (`KismetMathLibrary.Vector_Up`) (* DeltaSeconds (`self.CurrentSpeed`))) true)
  (if (and (< (`self.CurrentSpeed`) 0.0) (< _returnvalue_z _initiallocation_z))
    (`self.K2_SetActorLocation` (`self.InitialLocation`) false true)
    (`self.SetActorTickEnabled` false)))

(event `self.ReceiveActorEndOverlap`
  (params (OtherActor :type "Actor Object Reference"))
  (bind (_returnvalue_x _returnvalue_y _returnvalue_z) (`KismetMathLibrary.BreakVector` (`self.K2_GetActorLocation`)))
  (bind (_returnvalue_x_2 _returnvalue_y_2 _returnvalue_z_2) (`KismetMathLibrary.BreakVector` (`self.K2_GetActorLocation` OtherActor)))
  (bind (_returnvalue_x_3 _returnvalue_y_3) (`KismetMathLibrary.BreakVector` (`self.K2_GetActorLocation` OtherActor)))
  (bind (_returnvalue_x_4 _returnvalue_y_4 _returnvalue_z_3) (`KismetMathLibrary.BreakVector` (`self.K2_GetActorLocation`)))
  (`/Engine/EditorBlueprintResources/StandardMacros.IsValid` (`self.GetComponentByClass` OtherActor "/Script/Bonk.BonkBonkableComponent")
    (:`Is Valid`
      (`NiagaraFunctionLibrary.SpawnSystemAtLocation` "/Game/Art/VFX/sA_StylizedMix/Fx/NS_WaterSplash_Once.NS_WaterSplash_Once" (`KismetMathLibrary.MakeVector` _returnvalue_x_3 _returnvalue_y_3 _returnvalue_z_3))
      (`GameplayStatics.PlaySoundAtLocation` "/Game/SoundEffects/WaterSplash.WaterSplash" (`self.K2_GetActorLocation`) (struct) 0.09 1.0 0.0 null null null null)
      (bind _asbonk_player_pawn (cast `BonkPlayerPawn` OtherActor))
      (if (< _returnvalue_z_2 _returnvalue_z)
        (`self.K2_DestroyActor` _asbonk_player_pawn)))))

(event `OnRoundEnd_Event_0`
  (params (RoundNumber :type Integer))
  (set `self.bRoundEnded` true)
  (`self.OnDeactivate`)
  (`KismetSystemLibrary.K2_ClearAndInvalidateTimerHandle` (`self.LoweringTimerHandle`))
  (`KismetSystemLibrary.K2_ClearAndInvalidateTimerHandle` (`self.RaisingTimerHandle`)))

(event `OnRoundStart_Event_0`
  (params (RoundNumber :type Integer))
  (set `self.bRoundEnded` false)
  (bind _returnvalue (`KismetSystemLibrary.K2_SetTimerDelegate` (`|CreateDelegate` :!event `StartRaising`) (`self.TimeBeforeRaising`)))
  (set `self.RaisingTimerHandle` _returnvalue)
  (`KismetSystemLibrary.K2_ClearAndInvalidateTimerHandle` (`self.LoweringTimerHandle`)))

(event `StartRaising`
  (bind (_targetlocation_x _targetlocation_y _targetlocation_z) (`KismetMathLibrary.BreakVector` (`self.TargetLocation`)))
  (bind (_initiallocation_x _initiallocation_y _initiallocation_z) (`KismetMathLibrary.BreakVector` (`self.InitialLocation`)))
  (set `self.CurrentSpeed` (/ (`KismetMathLibrary.Abs` (- _targetlocation_z _initiallocation_z)) (`self.TimeToRaise`)))
  (`self.SetActorTickEnabled` true))

(event `StartLowering`
  (set `self.CurrentSpeed` (* (`self.DefaultRaisingSpeed`) -1.0))
  (`KismetSystemLibrary.K2_ClearAndInvalidateTimerHandle` (`self.LoweringTimerHandle`))
  (`KismetSystemLibrary.K2_ClearAndInvalidateTimerHandle` (`self.RaisingTimerHandle`)))

(fn `UserConstructionScript`
  (bind _targetlocation (`self.TargetLocation`))
  (`KismetSystemLibrary.DrawDebugPlane` (`KismetMathLibrary.MakePlaneFromPointAndNormal` _targetlocation (0.0 0.0 1.0)) _targetlocation 10000.0 (struct :`G` 0.113331 :`B` 1.0 :`A` 1.0) 1.0))