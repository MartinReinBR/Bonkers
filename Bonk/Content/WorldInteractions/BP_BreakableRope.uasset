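; BP_BreakableRope is a rope actor that suspends or tethers an assigned object and releases it when the rope takes any damage.
; On BeginPlay it constrains the target's static mesh with a physics constraint and attaches a cable component's end to that mesh.
; Damage calls DetachRope, which wakes the constrained body, breaks the constraint and frees the cable end.
; The construction script draws a debug line to the target for placement feedback.
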(event `self.ReceiveBeginPlay`
  (bind _returnvalue (`self.GetComponentByClass` (`self.ObjectToAttach`) "/Script/Engine.StaticMeshComponent"))
  (add `self.OnTakeAnyDamage` (delegate `OnTakeAnyDamage_Event_0`))
  (`PhysicsConstraintComponent.SetConstrainedComponents` (`self.PhysicsConstraint`) null "None" _returnvalue "None")
  (`CableComponent.SetAttachEndToComponent` (`self.Cable`) _returnvalue "None")
  (set `CableComponent.bAttachEnd` true (`self.Cable`)))

(event `OnTakeAnyDamage_Event_0` :!signature `self.OnTakeAnyDamage`
  (params (DamagedActor :type "Actor Object Reference") (Damage :type "Float (single-precision)") (DamageType :type "DamageType Object Reference") (InstigatedBy :type "Controller Object Reference") (DamageCauser :type "Actor Object Reference"))
  (`self.DetachRope`))

(fn `DetachRope`
  (bind (_outcomponent1 _outbonename1 _outcomponent2) (`PhysicsConstraintComponent.GetConstrainedComponents` (`self.PhysicsConstraint`)))
  (`/Engine/EditorBlueprintResources/StandardMacros.IsValid` _outcomponent2
    (:`Is Valid`
      (`PrimitiveComponent.WakeAllRigidBodies` _outcomponent2))
    (:`Is Not Valid`
      _))
  (`PhysicsConstraintComponent.BreakConstraint` (`self.PhysicsConstraint`))
  (set `CableComponent.bAttachEnd` false (`self.Cable`)))

(fn `UserConstructionScript`
  (bind _objecttoattach (`self.ObjectToAttach`))
  (`/Engine/EditorBlueprintResources/StandardMacros.IsValid` _objecttoattach
    (:`Is Valid`
      (`KismetSystemLibrary.DrawDebugLine` (`self.K2_GetActorLocation`) (`self.K2_GetActorLocation` _objecttoattach) (struct :`G` 0.163426 :`B` 1.0 :`A` 1.0) 3.0 5.0))))