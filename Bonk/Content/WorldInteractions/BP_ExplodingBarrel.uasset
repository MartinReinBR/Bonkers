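; Destructible exploding barrel that tracks its own health and detonates when damage brings it to zero.
; On detonation it applies strain and radial falloff force through a field system, deals full radial damage using the incoming damage type, then destroys itself.
; One radius and one magnitude drive both the field effects and the damage.
; Debug spheres show the blast radius at construction and on explosion.
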(event `self.ReceiveBeginPlay`
  (set `self.CurrentHealth` (`self.MaxHealth`))
  (add `self.OnTakeAnyDamage` (delegate `OnTakeDamage`)))

(event `OnTakeDamage` :!signature `self.OnTakeAnyDamage`
  (params (DamagedActor :type "Actor Object Reference") (Damage :type "Float (single-precision)") (DamageType :type "DamageType Object Reference") (InstigatedBy :type "Controller Object Reference") (DamageCauser :type "Actor Object Reference"))
  (bind _returnvalue (`self.K2_GetActorLocation`))
  (bind _output_get (set `self.CurrentHealth` (- (`self.CurrentHealth`) Damage)))
  (if (<= _output_get 0.0)
    (`self.ApplyEnvironmentReaction` _returnvalue (`self.ExplosionRadius`) (`self.ExplosionMagnitude`))
    (`GameplayStatics.ApplyRadialDamage` (`self.ExplosionMagnitude`) _returnvalue (`self.ExplosionRadius`) "/Script/Engine.DamageType" (`|MakeArray` self :!type "Actor Object Reference") null null true)
    (`KismetSystemLibrary.DrawDebugSphere` _returnvalue (`self.ExplosionRadius`) 12 (struct :`R` 1.0 :`B` 0.088168 :`A` 1.0) 5.0)
    (`self.K2_DestroyActor`)))

(fn `UserConstructionScript`
  (`KismetSystemLibrary.DrawDebugSphere` (`self.K2_GetActorLocation`) (`self.ExplosionRadius`) 12 (struct :`R` 1.0 :`A` 1.0) 1.0))